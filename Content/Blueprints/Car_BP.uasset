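; Car actor that acts as a lethal hazard: contact between any of its four wheels and the player character ends the game.
; All four wheel overlap events share one handler that checks whether the overlapping actor is the player's ThirdPersonCharacter.
; On a match it launches the character forward and upward along the car mesh's heading, enables ragdoll physics, deactivates movement, and shows GameOver_UI with UI-only mouse input.
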(event OnComponentBeginOverlap(Wheel_F_R)
  (params (OverlappedComponent :type Primitive%20Component%20Object%20Reference) (OtherActor :type Actor%20Object%20Reference) (OtherComp :type Primitive%20Component%20Object%20Reference) (OtherBodyIndex :type Integer) (bFromSweep :type Boolean) (SweepResult :type Hit%20Result%20Structure%20%28by%20ref%29))
  (bind _returnvalue (Game|GetPlayerController 0))
  (bind _mesh (Variables|Character|GetMesh))
  (bind _returnvalue_2 (Math|Vector|GetForwardVector _mesh))
  (bind (_x _y _z) (Math|Vector|BreakVector _returnvalue_2))
  (bind _asthird_person_character (Utilities|Casting|CastToThirdPersonCharacter (Game|GetPlayerCharacter 0))
    (:then
      (if (Math|Boolean|ORBoolean (== _asthird_person_character OtherActor) (== _asthird_person_character (stale OnComponentBeginOverlap(Wheel_F_L) OtherActor)) (== _asthird_person_character (stale OnComponentBeginOverlap(Wheel_B_L) OtherActor)) (== _asthird_person_character (stale OnComponentBeginOverlap(Wheel_B_R) OtherActor)))
        (Character|LaunchCharacter _asthird_person_character (* (Math|Vector|MakeVector _x _y (+ _z 1.0)) 1e+02) false false)
        (Physics|SetSimulatePhysics (Variables|/Script/Engine.Character|GetMesh _asthird_person_character) true)
        (Components|Activation|Deactivate (Variables|/Script/Engine.Character|GetCharacterMovement _asthird_person_character))
        (bind _returnvalue_3 (UserInterface|CreateWidget "/Game/Blueprints/GameOver_UI.GameOver_UI_C"))
        (bind _output_get (Variables|Default|SetGameOver_UI _returnvalue_3))
        (Variables|/Script/Engine.PlayerController|SetbShowMouseCursor _returnvalue true)
        (Input|SetInputModeUIOnly _returnvalue _output_get "DoNotLock")
        (Viewport|RemoveAllWidgets _output_get)
        (UserInterface|Viewport|AddtoViewport _output_get 0)))
    (:CastFailed
      (Development|PrintString "Cast Fail"))))

(event OnComponentBeginOverlap(Wheel_F_L)
  (params (OverlappedComponent :type Primitive%20Component%20Object%20Reference) (OtherActor :type Actor%20Object%20Reference) (OtherComp :type Primitive%20Component%20Object%20Reference) (OtherBodyIndex :type Integer) (bFromSweep :type Boolean) (SweepResult :type Hit%20Result%20Structure%20%28by%20ref%29))
  (bind _returnvalue (Game|GetPlayerController 0))
  (bind _mesh (Variables|Character|GetMesh))
  (bind _returnvalue_2 (Math|Vector|GetForwardVector _mesh))
  (bind (_x _y _z) (Math|Vector|BreakVector _returnvalue_2))
  (bind _asthird_person_character (Utilities|Casting|CastToThirdPersonCharacter (Game|GetPlayerCharacter 0))
    (:then
      (if (Math|Boolean|ORBoolean (== _asthird_person_character (stale OnComponentBeginOverlap(Wheel_F_R) OtherActor)) (== _asthird_person_character OtherActor) (== _asthird_person_character (stale OnComponentBeginOverlap(Wheel_B_L) OtherActor)) (== _asthird_person_character (stale OnComponentBeginOverlap(Wheel_B_R) OtherActor)))
        (Character|LaunchCharacter _asthird_person_character (* (Math|Vector|MakeVector _x _y (+ _z 1.0)) 1e+02) false false)
        (Physics|SetSimulatePhysics (Variables|/Script/Engine.Character|GetMesh _asthird_person_character) true)
        (Components|Activation|Deactivate (Variables|/Script/Engine.Character|GetCharacterMovement _asthird_person_character))
        (bind _returnvalue_3 (UserInterface|CreateWidget "/Game/Blueprints/GameOver_UI.GameOver_UI_C"))
        (bind _output_get (Variables|Default|SetGameOver_UI _returnvalue_3))
        (Variables|/Script/Engine.PlayerController|SetbShowMouseCursor _returnvalue true)
        (Input|SetInputModeUIOnly _returnvalue _output_get "DoNotLock")
        (Viewport|RemoveAllWidgets _output_get)
        (UserInterface|Viewport|AddtoViewport _output_get 0)))
    (:CastFailed
      (Development|PrintString "Cast Fail"))))

(event OnComponentBeginOverlap(Wheel_B_L)
  (params (OverlappedComponent :type Primitive%20Component%20Object%20Reference) (OtherActor :type Actor%20Object%20Reference) (OtherComp :type Primitive%20Component%20Object%20Reference) (OtherBodyIndex :type Integer) (bFromSweep :type Boolean) (SweepResult :type Hit%20Result%20Structure%20%28by%20ref%29))
  (bind _returnvalue (Game|GetPlayerController 0))
  (bind _mesh (Variables|Character|GetMesh))
  (bind _returnvalue_2 (Math|Vector|GetForwardVector _mesh))
  (bind (_x _y _z) (Math|Vector|BreakVector _returnvalue_2))
  (bind _asthird_person_character (Utilities|Casting|CastToThirdPersonCharacter (Game|GetPlayerCharacter 0))
    (:then
      (if (Math|Boolean|ORBoolean (== _asthird_person_character (stale OnComponentBeginOverlap(Wheel_F_R) OtherActor)) (== _asthird_person_character (stale OnComponentBeginOverlap(Wheel_F_L) OtherActor)) (== _asthird_person_character OtherActor) (== _asthird_person_character (stale OnComponentBeginOverlap(Wheel_B_R) OtherActor)))
        (Character|LaunchCharacter _asthird_person_character (* (Math|Vector|MakeVector _x _y (+ _z 1.0)) 1e+02) false false)
        (Physics|SetSimulatePhysics (Variables|/Script/Engine.Character|GetMesh _asthird_person_character) true)
        (Components|Activation|Deactivate (Variables|/Script/Engine.Character|GetCharacterMovement _asthird_person_character))
        (bind _returnvalue_3 (UserInterface|CreateWidget "/Game/Blueprints/GameOver_UI.GameOver_UI_C"))
        (bind _output_get (Variables|Default|SetGameOver_UI _returnvalue_3))
        (Variables|/Script/Engine.PlayerController|SetbShowMouseCursor _returnvalue true)
        (Input|SetInputModeUIOnly _returnvalue _output_get "DoNotLock")
        (Viewport|RemoveAllWidgets _output_get)
        (UserInterface|Viewport|AddtoViewport _output_get 0)))
    (:CastFailed
      (Development|PrintString "Cast Fail"))))

(event OnComponentBeginOverlap(Wheel_B_R)
  (params (OverlappedComponent :type Primitive%20Component%20Object%20Reference) (OtherActor :type Actor%20Object%20Reference) (OtherComp :type Primitive%20Component%20Object%20Reference) (OtherBodyIndex :type Integer) (bFromSweep :type Boolean) (SweepResult :type Hit%20Result%20Structure%20%28by%20ref%29))
  (bind _returnvalue (Game|GetPlayerController 0))
  (bind _mesh (Variables|Character|GetMesh))
  (bind _returnvalue_2 (Math|Vector|GetForwardVector _mesh))
  (bind (_x _y _z) (Math|Vector|BreakVector _returnvalue_2))
  (bind _asthird_person_character (Utilities|Casting|CastToThirdPersonCharacter (Game|GetPlayerCharacter 0))
    (:then
      (if (Math|Boolean|ORBoolean (== _asthird_person_character (stale OnComponentBeginOverlap(Wheel_F_R) OtherActor)) (== _asthird_person_character (stale OnComponentBeginOverlap(Wheel_F_L) OtherActor)) (== _asthird_person_character (stale OnComponentBeginOverlap(Wheel_B_L) OtherActor)) (== _asthird_person_character OtherActor))
        (Character|LaunchCharacter _asthird_person_character (* (Math|Vector|MakeVector _x _y (+ _z 1.0)) 1e+02) false false)
        (Physics|SetSimulatePhysics (Variables|/Script/Engine.Character|GetMesh _asthird_person_character) true)
        (Components|Activation|Deactivate (Variables|/Script/Engine.Character|GetCharacterMovement _asthird_person_character))
        (bind _returnvalue_3 (UserInterface|CreateWidget "/Game/Blueprints/GameOver_UI.GameOver_UI_C"))
        (bind _output_get (Variables|Default|SetGameOver_UI _returnvalue_3))
        (Variables|/Script/Engine.PlayerController|SetbShowMouseCursor _returnvalue true)
        (Input|SetInputModeUIOnly _returnvalue _output_get "DoNotLock")
        (Viewport|RemoveAllWidgets _output_get)
        (UserInterface|Viewport|AddtoViewport _output_get 0)))
    (:CastFailed
      (Development|PrintString "Cast Fail"))))

(event EventBeginPlay)

(event Collision|EventActorBeginOverlap
  (params (OtherActor :type Actor%20Object%20Reference)))

(event EventTick
  (params (DeltaSeconds :type Float%20%28single-precision%29)))

(fn ConstructionScript)