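; Car hazard actor that kills baby turtles and the player when any of its four wheels overlaps them.
; All wheel overlaps share one handler, which replaces a hit Baby_BP with a dead-turtle sprite actor.
; A living player ragdolls, gets launched along the car's forward vector with a brake sound, is marked dead and loses movement.
; The player's death then opens the Game Over widget with mouse cursor and UI-only input.
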(event OnComponentBeginOverlap(Wheel_F_R)
  (params (OverlappedComponent :type Primitive%20Component%20Object%20Reference) (OtherActor :type Actor%20Object%20Reference) (OtherComp :type Primitive%20Component%20Object%20Reference) (OtherBodyIndex :type Integer) (bFromSweep :type Boolean) (SweepResult :type Hit%20Result%20Structure%20%28by%20ref%29))
  (bind _returnvalue (Game|GetPlayerController 0))
  (bind _returnvalue_2 (Game|GetPlayerCharacter 0))
  (if (Math|Boolean|ORBoolean (== (Utilities|GetClass OtherActor) "/Game/Blueprints/Actors/Baby_BP.Baby_BP_C") (== (Utilities|GetClass (stale OnComponentBeginOverlap(Wheel_F_L) OtherActor)) "/Game/Blueprints/Actors/Baby_BP.Baby_BP_C") (== (Utilities|GetClass (stale OnComponentBeginOverlap(Wheel_B_L) OtherActor)) "/Game/Blueprints/Actors/Baby_BP.Baby_BP_C") (== (Utilities|GetClass (stale OnComponentBeginOverlap(Wheel_B_R) OtherActor)) "/Game/Blueprints/Actors/Baby_BP.Baby_BP_C"))
    (bind _outactors (Actor|GetAllActorsOfClass "/Game/Blueprints/Actors/Baby_BP.Baby_BP_C"))
    (for _array_element _outactors
      (if (Math|Boolean|ORBoolean (== _array_element OtherActor) (== _array_element (stale OnComponentBeginOverlap(Wheel_F_L) OtherActor)) (== _array_element (stale OnComponentBeginOverlap(Wheel_B_L) OtherActor)) (== _array_element (stale OnComponentBeginOverlap(Wheel_B_R) OtherActor)))
        (Physics|SetSimulatePhysics (Variables|/Script/Engine.Character|GetMesh _array_element) true)
        (Utilities|Casting|CastToThirdPersonCharacter (Game|GetPlayerCharacter 0))
        (Game|SpawnActorfromClass "/Game/Blueprints/Actors/DeadTurtle_Sprite_BP.DeadTurtle_Sprite_BP_C" (Utilities|SpriteTransform (Transformation|GetActorTransform _array_element)) "Undefined" 0 0)
        (Actor|DestroyActor _array_element)))
    (else
      (bind _asthird_person_character (Utilities|Casting|CastToThirdPersonCharacter _returnvalue_2))
      (if (not (Variables|/Game/Blueprints/Actors/ThirdPersonCharacter.ThirdPersonCharacter_C|GetPlayerIsDead _asthird_person_character))
        (if (Math|Boolean|ORBoolean (== _asthird_person_character OtherActor) (== _asthird_person_character (stale OnComponentBeginOverlap(Wheel_F_L) OtherActor)) (== _asthird_person_character (stale OnComponentBeginOverlap(Wheel_B_L) OtherActor)) (== _asthird_person_character (stale OnComponentBeginOverlap(Wheel_B_R) OtherActor)))
          (Physics|SetSimulatePhysics (Variables|/Script/Engine.Character|GetMesh _asthird_person_character) true)
          (Audio|PlaySoundatLocation "/Game/Sounds/CarBrake.CarBrake" (Transformation|GetActorLocation _returnvalue_2) "0, 0, 0" 1.0 1.0 0.3)
          (Physics|AddImpulse (Variables|/Script/Engine.Character|GetMesh _asthird_person_character) (* (Math|Vector|GetForwardVector (Variables|Character|GetMesh)) 1e+03) "None" false)
          (Variables|/Game/Blueprints/Actors/ThirdPersonCharacter.ThirdPersonCharacter_C|SetPlayerIsDead _asthird_person_character true)
          (Components|Activation|Deactivate (Variables|/Script/Engine.Character|GetCharacterMovement _asthird_person_character))
          (bind _returnvalue_3 (UserInterface|CreateWidget "/Game/Blueprints/UI/GameOver_UI.GameOver_UI_C"))
          (bind _output_get (Variables|Default|SetGameOver_UI _returnvalue_3))
          (Variables|/Script/Engine.PlayerController|SetbShowMouseCursor _returnvalue true)
          (Input|SetInputModeUIOnly _returnvalue _output_get "DoNotLock")
          (Viewport|RemoveAllWidgets _output_get)
          (UserInterface|Viewport|AddtoViewport _output_get 0))))))

(event OnComponentBeginOverlap(Wheel_F_L)
  (params (OverlappedComponent :type Primitive%20Component%20Object%20Reference) (OtherActor :type Actor%20Object%20Reference) (OtherComp :type Primitive%20Component%20Object%20Reference) (OtherBodyIndex :type Integer) (bFromSweep :type Boolean) (SweepResult :type Hit%20Result%20Structure%20%28by%20ref%29))
  (bind _returnvalue (Game|GetPlayerController 0))
  (bind _returnvalue_2 (Game|GetPlayerCharacter 0))
  (if (Math|Boolean|ORBoolean (== (Utilities|GetClass (stale OnComponentBeginOverlap(Wheel_F_R) OtherActor)) "/Game/Blueprints/Actors/Baby_BP.Baby_BP_C") (== (Utilities|GetClass OtherActor) "/Game/Blueprints/Actors/Baby_BP.Baby_BP_C") (== (Utilities|GetClass (stale OnComponentBeginOverlap(Wheel_B_L) OtherActor)) "/Game/Blueprints/Actors/Baby_BP.Baby_BP_C") (== (Utilities|GetClass (stale OnComponentBeginOverlap(Wheel_B_R) OtherActor)) "/Game/Blueprints/Actors/Baby_BP.Baby_BP_C"))
    (bind _outactors (Actor|GetAllActorsOfClass "/Game/Blueprints/Actors/Baby_BP.Baby_BP_C"))
    (for _array_element _outactors
      (if (Math|Boolean|ORBoolean (== _array_element (stale OnComponentBeginOverlap(Wheel_F_R) OtherActor)) (== _array_element OtherActor) (== _array_element (stale OnComponentBeginOverlap(Wheel_B_L) OtherActor)) (== _array_element (stale OnComponentBeginOverlap(Wheel_B_R) OtherActor)))
        (Physics|SetSimulatePhysics (Variables|/Script/Engine.Character|GetMesh _array_element) true)
        (Utilities|Casting|CastToThirdPersonCharacter (Game|GetPlayerCharacter 0))
        (Game|SpawnActorfromClass "/Game/Blueprints/Actors/DeadTurtle_Sprite_BP.DeadTurtle_Sprite_BP_C" (Utilities|SpriteTransform (Transformation|GetActorTransform _array_element)) "Undefined" 0 0)
        (Actor|DestroyActor _array_element)))
    (else
      (bind _asthird_person_character (Utilities|Casting|CastToThirdPersonCharacter _returnvalue_2))
      (if (not (Variables|/Game/Blueprints/Actors/ThirdPersonCharacter.ThirdPersonCharacter_C|GetPlayerIsDead _asthird_person_character))
        (if (Math|Boolean|ORBoolean (== _asthird_person_character (stale OnComponentBeginOverlap(Wheel_F_R) OtherActor)) (== _asthird_person_character OtherActor) (== _asthird_person_character (stale OnComponentBeginOverlap(Wheel_B_L) OtherActor)) (== _asthird_person_character (stale OnComponentBeginOverlap(Wheel_B_R) OtherActor)))
          (Physics|SetSimulatePhysics (Variables|/Script/Engine.Character|GetMesh _asthird_person_character) true)
          (Audio|PlaySoundatLocation "/Game/Sounds/CarBrake.CarBrake" (Transformation|GetActorLocation _returnvalue_2) "0, 0, 0" 1.0 1.0 0.3)
          (Physics|AddImpulse (Variables|/Script/Engine.Character|GetMesh _asthird_person_character) (* (Math|Vector|GetForwardVector (Variables|Character|GetMesh)) 1e+03) "None" false)
          (Variables|/Game/Blueprints/Actors/ThirdPersonCharacter.ThirdPersonCharacter_C|SetPlayerIsDead _asthird_person_character true)
          (Components|Activation|Deactivate (Variables|/Script/Engine.Character|GetCharacterMovement _asthird_person_character))
          (bind _returnvalue_3 (UserInterface|CreateWidget "/Game/Blueprints/UI/GameOver_UI.GameOver_UI_C"))
          (bind _output_get (Variables|Default|SetGameOver_UI _returnvalue_3))
          (Variables|/Script/Engine.PlayerController|SetbShowMouseCursor _returnvalue true)
          (Input|SetInputModeUIOnly _returnvalue _output_get "DoNotLock")
          (Viewport|RemoveAllWidgets _output_get)
          (UserInterface|Viewport|AddtoViewport _output_get 0))))))

(event OnComponentBeginOverlap(Wheel_B_L)
  (params (OverlappedComponent :type Primitive%20Component%20Object%20Reference) (OtherActor :type Actor%20Object%20Reference) (OtherComp :type Primitive%20Component%20Object%20Reference) (OtherBodyIndex :type Integer) (bFromSweep :type Boolean) (SweepResult :type Hit%20Result%20Structure%20%28by%20ref%29))
  (bind _returnvalue (Game|GetPlayerController 0))
  (bind _returnvalue_2 (Game|GetPlayerCharacter 0))
  (if (Math|Boolean|ORBoolean (== (Utilities|GetClass (stale OnComponentBeginOverlap(Wheel_F_R) OtherActor)) "/Game/Blueprints/Actors/Baby_BP.Baby_BP_C") (== (Utilities|GetClass (stale OnComponentBeginOverlap(Wheel_F_L) OtherActor)) "/Game/Blueprints/Actors/Baby_BP.Baby_BP_C") (== (Utilities|GetClass OtherActor) "/Game/Blueprints/Actors/Baby_BP.Baby_BP_C") (== (Utilities|GetClass (stale OnComponentBeginOverlap(Wheel_B_R) OtherActor)) "/Game/Blueprints/Actors/Baby_BP.Baby_BP_C"))
    (bind _outactors (Actor|GetAllActorsOfClass "/Game/Blueprints/Actors/Baby_BP.Baby_BP_C"))
    (for _array_element _outactors
      (if (Math|Boolean|ORBoolean (== _array_element (stale OnComponentBeginOverlap(Wheel_F_R) OtherActor)) (== _array_element (stale OnComponentBeginOverlap(Wheel_F_L) OtherActor)) (== _array_element OtherActor) (== _array_element (stale OnComponentBeginOverlap(Wheel_B_R) OtherActor)))
        (Physics|SetSimulatePhysics (Variables|/Script/Engine.Character|GetMesh _array_element) true)
        (Utilities|Casting|CastToThirdPersonCharacter (Game|GetPlayerCharacter 0))
        (Game|SpawnActorfromClass "/Game/Blueprints/Actors/DeadTurtle_Sprite_BP.DeadTurtle_Sprite_BP_C" (Utilities|SpriteTransform (Transformation|GetActorTransform _array_element)) "Undefined" 0 0)
        (Actor|DestroyActor _array_element)))
    (else
      (bind _asthird_person_character (Utilities|Casting|CastToThirdPersonCharacter _returnvalue_2))
      (if (not (Variables|/Game/Blueprints/Actors/ThirdPersonCharacter.ThirdPersonCharacter_C|GetPlayerIsDead _asthird_person_character))
        (if (Math|Boolean|ORBoolean (== _asthird_person_character (stale OnComponentBeginOverlap(Wheel_F_R) OtherActor)) (== _asthird_person_character (stale OnComponentBeginOverlap(Wheel_F_L) OtherActor)) (== _asthird_person_character OtherActor) (== _asthird_person_character (stale OnComponentBeginOverlap(Wheel_B_R) OtherActor)))
          (Physics|SetSimulatePhysics (Variables|/Script/Engine.Character|GetMesh _asthird_person_character) true)
          (Audio|PlaySoundatLocation "/Game/Sounds/CarBrake.CarBrake" (Transformation|GetActorLocation _returnvalue_2) "0, 0, 0" 1.0 1.0 0.3)
          (Physics|AddImpulse (Variables|/Script/Engine.Character|GetMesh _asthird_person_character) (* (Math|Vector|GetForwardVector (Variables|Character|GetMesh)) 1e+03) "None" false)
          (Variables|/Game/Blueprints/Actors/ThirdPersonCharacter.ThirdPersonCharacter_C|SetPlayerIsDead _asthird_person_character true)
          (Components|Activation|Deactivate (Variables|/Script/Engine.Character|GetCharacterMovement _asthird_person_character))
          (bind _returnvalue_3 (UserInterface|CreateWidget "/Game/Blueprints/UI/GameOver_UI.GameOver_UI_C"))
          (bind _output_get (Variables|Default|SetGameOver_UI _returnvalue_3))
          (Variables|/Script/Engine.PlayerController|SetbShowMouseCursor _returnvalue true)
          (Input|SetInputModeUIOnly _returnvalue _output_get "DoNotLock")
          (Viewport|RemoveAllWidgets _output_get)
          (UserInterface|Viewport|AddtoViewport _output_get 0))))))

(event OnComponentBeginOverlap(Wheel_B_R)
  (params (OverlappedComponent :type Primitive%20Component%20Object%20Reference) (OtherActor :type Actor%20Object%20Reference) (OtherComp :type Primitive%20Component%20Object%20Reference) (OtherBodyIndex :type Integer) (bFromSweep :type Boolean) (SweepResult :type Hit%20Result%20Structure%20%28by%20ref%29))
  (bind _returnvalue (Game|GetPlayerController 0))
  (bind _returnvalue_2 (Game|GetPlayerCharacter 0))
  (if (Math|Boolean|ORBoolean (== (Utilities|GetClass (stale OnComponentBeginOverlap(Wheel_F_R) OtherActor)) "/Game/Blueprints/Actors/Baby_BP.Baby_BP_C") (== (Utilities|GetClass (stale OnComponentBeginOverlap(Wheel_F_L) OtherActor)) "/Game/Blueprints/Actors/Baby_BP.Baby_BP_C") (== (Utilities|GetClass (stale OnComponentBeginOverlap(Wheel_B_L) OtherActor)) "/Game/Blueprints/Actors/Baby_BP.Baby_BP_C") (== (Utilities|GetClass OtherActor) "/Game/Blueprints/Actors/Baby_BP.Baby_BP_C"))
    (bind _outactors (Actor|GetAllActorsOfClass "/Game/Blueprints/Actors/Baby_BP.Baby_BP_C"))
    (for _array_element _outactors
      (if (Math|Boolean|ORBoolean (== _array_element (stale OnComponentBeginOverlap(Wheel_F_R) OtherActor)) (== _array_element (stale OnComponentBeginOverlap(Wheel_F_L) OtherActor)) (== _array_element (stale OnComponentBeginOverlap(Wheel_B_L) OtherActor)) (== _array_element OtherActor))
        (Physics|SetSimulatePhysics (Variables|/Script/Engine.Character|GetMesh _array_element) true)
        (Utilities|Casting|CastToThirdPersonCharacter (Game|GetPlayerCharacter 0))
        (Game|SpawnActorfromClass "/Game/Blueprints/Actors/DeadTurtle_Sprite_BP.DeadTurtle_Sprite_BP_C" (Utilities|SpriteTransform (Transformation|GetActorTransform _array_element)) "Undefined" 0 0)
        (Actor|DestroyActor _array_element)))
    (else
      (bind _asthird_person_character (Utilities|Casting|CastToThirdPersonCharacter _returnvalue_2))
      (if (not (Variables|/Game/Blueprints/Actors/ThirdPersonCharacter.ThirdPersonCharacter_C|GetPlayerIsDead _asthird_person_character))
        (if (Math|Boolean|ORBoolean (== _asthird_person_character (stale OnComponentBeginOverlap(Wheel_F_R) OtherActor)) (== _asthird_person_character (stale OnComponentBeginOverlap(Wheel_F_L) OtherActor)) (== _asthird_person_character (stale OnComponentBeginOverlap(Wheel_B_L) OtherActor)) (== _asthird_person_character OtherActor))
          (Physics|SetSimulatePhysics (Variables|/Script/Engine.Character|GetMesh _asthird_person_character) true)
          (Audio|PlaySoundatLocation "/Game/Sounds/CarBrake.CarBrake" (Transformation|GetActorLocation _returnvalue_2) "0, 0, 0" 1.0 1.0 0.3)
          (Physics|AddImpulse (Variables|/Script/Engine.Character|GetMesh _asthird_person_character) (* (Math|Vector|GetForwardVector (Variables|Character|GetMesh)) 1e+03) "None" false)
          (Variables|/Game/Blueprints/Actors/ThirdPersonCharacter.ThirdPersonCharacter_C|SetPlayerIsDead _asthird_person_character true)
          (Components|Activation|Deactivate (Variables|/Script/Engine.Character|GetCharacterMovement _asthird_person_character))
          (bind _returnvalue_3 (UserInterface|CreateWidget "/Game/Blueprints/UI/GameOver_UI.GameOver_UI_C"))
          (bind _output_get (Variables|Default|SetGameOver_UI _returnvalue_3))
          (Variables|/Script/Engine.PlayerController|SetbShowMouseCursor _returnvalue true)
          (Input|SetInputModeUIOnly _returnvalue _output_get "DoNotLock")
          (Viewport|RemoveAllWidgets _output_get)
          (UserInterface|Viewport|AddtoViewport _output_get 0))))))

(event EventBeginPlay)

(event Collision|EventActorBeginOverlap
  (params (OtherActor :type Actor%20Object%20Reference)))

(event EventTick
  (params (DeltaSeconds :type Float%20%28single-precision%29)))

(fn ConstructionScript)